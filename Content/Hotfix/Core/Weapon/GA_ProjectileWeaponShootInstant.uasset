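; Gameplay ability for an instant weapon shot that spawns a projectile from the avatar character.
; After committing, it builds an effect container spec and assigns Damage to the first target effect spec as a set-by-caller magnitude.
; It spawns ProjectileClass at the avatar's location and rotation, passing the container and the character as owner and instigator.
; The ability ends right after spawning, or cancels if the commit fails.
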(event Ability|EventActivateAbility
  (bind _returnvalue (Ability|GetAvatarActorfromActorInfo))
  (bind _returnvalue_2 (Ability|CommitAbility))
  (if _returnvalue_2
    (bind _returnvalue_3 (Class|GASGameplayAbility|MakeEffectContainerSpec))
    (Ability|GameplayEffect|AssignTagSetbyCallerMagnitude :SpecHandle (Utilities|Array|Get(acopy) (.TargetGameplayEffectSpecs (Utilities|Struct|BreakGASEffectContainerSpec _returnvalue_3))) :Magnitude (Variables|Default|GetDamage))
    (bind _asgame_character (Utilities|Casting|CastToGameCharacter (Ability|GetAvatarActorfromActorInfo)))
    (Game|SpawnActorfromClass (Variables|Default|GetProjectileClass) (Math|Transform|MakeTransform (Transformation|GetActorLocation _returnvalue) (Transformation|GetActorRotation _returnvalue) "1,1,1") "Undefined" _asgame_character _returnvalue_3 _asgame_character)
    (Ability|EndAbility)
    (else
      (Ability|CancelAbility))))